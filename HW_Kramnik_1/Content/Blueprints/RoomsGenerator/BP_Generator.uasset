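; Room generator trigger that streams in the next pair of rooms when the player character first overlaps it.
; Each trigger updates the character's room counters, then loads level instances at two offsets from its Box.
; While rooms remain, Easy and Hard levels swap slots randomly and BPActorSpawn runs the matching spawn function; otherwise both slots get LevelEnd.
; An unconnected branch holds an unused random End/Hard variant.
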(event `self.ReceiveActorBeginOverlap`
  (params (OtherActor :type "Actor Object Reference"))
  (bind _bp_actorspawn (`self.BP_ActorSpawn`))
  (bind _asbp_third_person_character (cast `/Game/ThirdPerson/Blueprints/BP_ThirdPersonCharacter` OtherActor))
  (`/Engine/EditorBlueprintResources/StandardMacros.DoOnce` false ; Позволяет сделать все один раз
    (:`Completed`
      (set `/Game/ThirdPerson/Blueprints/BP_ThirdPersonCharacter.CounterOfRooms` (+ (`/Game/ThirdPerson/Blueprints/BP_ThirdPersonCharacter.CounterOfRooms` _asbp_third_person_character) 1) _asbp_third_person_character)
      (bind _output_get (set `/Game/ThirdPerson/Blueprints/BP_ThirdPersonCharacter.HowManyRooms?` (- (`/Game/ThirdPerson/Blueprints/BP_ThirdPersonCharacter.HowManyRooms?` _asbp_third_person_character) 1) _asbp_third_person_character)) ; Обновлеят, сколько комнат осталось до конца
      (if (<= _output_get 0)
        ;[1 1 1] Генерация LevelEnd
        (`LevelStreamingDynamic.LoadLevelInstanceBySoftObjectPtr` "/Game/AllLevels/LevelEnd.LevelEnd" (+ (`SceneComponent.K2_GetComponentLocation` (`self.Box`)) (`self.Place_1`)) (struct :`Yaw` 180.0) "" null)
        (`LevelStreamingDynamic.LoadLevelInstanceBySoftObjectPtr` "/Game/AllLevels/LevelEnd.LevelEnd" (+ (`SceneComponent.K2_GetComponentLocation` (`self.Box`)) (`self.Place_2`)) (struct :`Yaw` 270.0) "" null)
        (elif (`KismetMathLibrary.RandomBool`)
          ;[1 1 1] Генерация LevelEasy и LevelHard
          (`LevelStreamingDynamic.LoadLevelInstanceBySoftObjectPtr` "/Game/AllLevels/LevelEasy.LevelEasy" (+ (`SceneComponent.K2_GetComponentLocation` (`self.Box`)) (`self.Place_1`)) (struct :`Yaw` 180.0) "" null)
          (`/Game/Blueprints/RoomsGenerator/BP_ActorSpawn.LevelEasy_1` _bp_actorspawn)
          (`LevelStreamingDynamic.LoadLevelInstanceBySoftObjectPtr` "/Game/AllLevels/LevelHard.LevelHard" (+ (`SceneComponent.K2_GetComponentLocation` (`self.Box`)) (`self.Place_2`)) (struct :`Yaw` 90.0) "" null)
          (`/Game/Blueprints/RoomsGenerator/BP_ActorSpawn.LevelHard_2` _bp_actorspawn)
          (else
            (`LevelStreamingDynamic.LoadLevelInstanceBySoftObjectPtr` "/Game/AllLevels/LevelHard.LevelHard" (+ (`SceneComponent.K2_GetComponentLocation` (`self.Box`)) (`self.Place_1`)) (struct :`Yaw` 180.0) "" null)
            (`/Game/Blueprints/RoomsGenerator/BP_ActorSpawn.LevelHard_1` _bp_actorspawn)
            (`LevelStreamingDynamic.LoadLevelInstanceBySoftObjectPtr` "/Game/AllLevels/LevelEasy.LevelEasy" (+ (`SceneComponent.K2_GetComponentLocation` (`self.Box`)) (`self.Place_2`)) (struct :`Yaw` 90.0) "" null)
            (`/Game/Blueprints/RoomsGenerator/BP_ActorSpawn.LevelEasy_2` _bp_actorspawn)))))))

(fn `UserConstructionScript`)