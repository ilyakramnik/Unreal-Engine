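; BP_Destroy is a one-shot trigger in the room generator that updates door actors when the third-person character stops overlapping it.
; It flips the character's CounterOfDoors boolean, so successive triggers alternate behavior.
; When the flag was false it only destroys DoorOpen; when true it also moves DoorClose into the destroyed door's location.
; Either branch then destroys the trigger itself.
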(event `self.ReceiveActorEndOverlap`
  (params (OtherActor :type "Actor Object Reference"))
  (bind _dooropen (`self.DoorOpen`))
  (bind _asbp_third_person_character (cast `/Game/ThirdPerson/Blueprints/BP_ThirdPersonCharacter` OtherActor))
  (bind _counterofdoors (`/Game/ThirdPerson/Blueprints/BP_ThirdPersonCharacter.CounterOfDoors` _asbp_third_person_character))
  (`KismetSystemLibrary.PrintString` (`KismetStringLibrary.Conv_BoolToString` _counterofdoors))
  (if (== _counterofdoors false)
    (set `/Game/ThirdPerson/Blueprints/BP_ThirdPersonCharacter.CounterOfDoors` true _asbp_third_person_character)
    (`self.K2_DestroyActor` _dooropen)
    (`self.K2_DestroyActor`)
    (else
      (set `/Game/ThirdPerson/Blueprints/BP_ThirdPersonCharacter.CounterOfDoors` false _asbp_third_person_character)
      (bind _output_get (set `self.DoorLocation` (`self.K2_GetActorLocation` _dooropen)))
      (`self.K2_DestroyActor` _dooropen)
      (`self.K2_SetActorLocation` (`self.DoorClose`) _output_get false false)
      (`self.K2_DestroyActor`))))

(event `self.ReceiveActorBeginOverlap`
  (params (OtherActor :type "Actor Object Reference")))

(fn `UserConstructionScript`)