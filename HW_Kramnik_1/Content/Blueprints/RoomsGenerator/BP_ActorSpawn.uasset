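; BP_ActorSpawn populates generated rooms with buffs and traps through four events: easy and hard variants for each of two placements.
; Easy events spawn a buff picked from a list, while hard events always spawn BP_Buff_HP.
; The player character's CounterOfRooms drives randomized trap counts and slides the selection window through separate easy and hard trap lists.
; Everything spawns at random points within the Box extent, offset by Place1 or Place2.
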(event `LevelEasy_1`
  (bind _box (`self.Box`))
  (bind _returnvalue (`KismetMathLibrary.Conv_VectorToTransform` (`KismetMathLibrary.RandomPointInBoundingBox` (+ (`SceneComponent.K2_GetComponentLocation` _box) (`self.Place_1`)) (`BoxComponent.GetScaledBoxExtent` _box))))
  ;[1 1 1] Генерация одного из бафов
  (for _ (range (+ (`KismetMathLibrary.RandomInteger` 1) 1))
    (`|SpawnActorFromClass` (`|GetArrayItem` (`self.Class`) (`KismetMathLibrary.RandomIntegerInRange` 0 2)) _returnvalue "Undefined" "SelectDefaultAtRuntime" null null)
    ;[1 1 1] Генерация ловушек, которая зависит от количества пройденных комнат и от сложности предыдущей
    (bind _asbp_third_person_character (cast `/Game/ThirdPerson/Blueprints/BP_ThirdPersonCharacter` (`GameplayStatics.GetPlayerCharacter` 0)))
    (bind _counterofrooms (`/Game/ThirdPerson/Blueprints/BP_ThirdPersonCharacter.CounterOfRooms` _asbp_third_person_character))
    (bind _returnvalue_2 (+ _counterofrooms 2))
    (for _ (range (`KismetMathLibrary.RandomIntegerInRange` _returnvalue_2 _returnvalue_2) (+ (`KismetMathLibrary.RandomIntegerInRange` (+ _counterofrooms 5) (+ _counterofrooms 15)) 1))
      (`|SpawnActorFromClass` (`|GetArrayItem` (`self.Class_1`) (`KismetMathLibrary.RandomIntegerInRange` _counterofrooms (+ _counterofrooms 2))) _returnvalue "Undefined" "SelectDefaultAtRuntime" null null))))

(event `LevelEasy_2`
  (bind _box (`self.Box`))
  (bind _returnvalue (`KismetMathLibrary.Conv_VectorToTransform` (`KismetMathLibrary.RandomPointInBoundingBox` (+ (`SceneComponent.K2_GetComponentLocation` _box) (`self.Place_2`)) (`BoxComponent.GetScaledBoxExtent` _box))))
  ;[1 1 1] Генерация одного из бафов
  (for _ (range (+ (`KismetMathLibrary.RandomInteger` 1) 1))
    (`|SpawnActorFromClass` (`|GetArrayItem` (`self.Class`) (`KismetMathLibrary.RandomIntegerInRange` 0 2)) _returnvalue "Undefined" "SelectDefaultAtRuntime" null null)
    ;[1 1 1] Генерация ловушек, которая зависит от количества пройденных комнат и от сложности предыдущей
    (bind _asbp_third_person_character (cast `/Game/ThirdPerson/Blueprints/BP_ThirdPersonCharacter` (`GameplayStatics.GetPlayerCharacter` 0)))
    (bind _counterofrooms (`/Game/ThirdPerson/Blueprints/BP_ThirdPersonCharacter.CounterOfRooms` _asbp_third_person_character))
    (bind _returnvalue_2 (+ _counterofrooms 2))
    (for _ (range (`KismetMathLibrary.RandomIntegerInRange` _returnvalue_2 _returnvalue_2) (+ (`KismetMathLibrary.RandomIntegerInRange` (+ _counterofrooms 5) (+ _counterofrooms 15)) 1))
      (`|SpawnActorFromClass` (`|GetArrayItem` (`self.Class_1`) (`KismetMathLibrary.RandomIntegerInRange` _counterofrooms (+ _counterofrooms 2))) _returnvalue "Undefined" "SelectDefaultAtRuntime" null null))))

(event `LevelHard_1`
  (bind _box (`self.Box`))
  (bind _returnvalue (`KismetMathLibrary.Conv_VectorToTransform` (`KismetMathLibrary.RandomPointInBoundingBox` (+ (`SceneComponent.K2_GetComponentLocation` _box) (`self.Place_1`)) (`BoxComponent.GetScaledBoxExtent` _box))))
  ;[1 1 1] Генерация BuffHP
  (`|SpawnActorFromClass` "/Game/Blueprints/Actors/BP_Buff_HP.BP_Buff_HP_C" _returnvalue "Undefined" "OverrideRootScale" null null)
  ;[1 1 1] Генерация ловушек, которая зависит от количества пройденных комнат и от сложности предыдущей
  (bind _asbp_third_person_character (cast `/Game/ThirdPerson/Blueprints/BP_ThirdPersonCharacter` (`GameplayStatics.GetPlayerCharacter` 0)))
  (bind _counterofrooms (`/Game/ThirdPerson/Blueprints/BP_ThirdPersonCharacter.CounterOfRooms` _asbp_third_person_character))
  (bind _returnvalue_2 (+ _counterofrooms 2))
  (for _ (range (`KismetMathLibrary.RandomIntegerInRange` _returnvalue_2 _returnvalue_2) (+ (`KismetMathLibrary.RandomIntegerInRange` (+ _counterofrooms 7) (+ _counterofrooms 15)) 1))
    (`|SpawnActorFromClass` (`|GetArrayItem` (`self.Class_0`) (`KismetMathLibrary.RandomIntegerInRange` _counterofrooms (+ _counterofrooms 2))) _returnvalue "Undefined" "SelectDefaultAtRuntime" null null)))

(event `LevelHard_2`
  (bind _box (`self.Box`))
  (bind _returnvalue (`KismetMathLibrary.Conv_VectorToTransform` (`KismetMathLibrary.RandomPointInBoundingBox` (+ (`SceneComponent.K2_GetComponentLocation` _box) (`self.Place_2`)) (`BoxComponent.GetScaledBoxExtent` _box))))
  ;[1 1 1] Генерация BuffHP
  (`|SpawnActorFromClass` "/Game/Blueprints/Actors/BP_Buff_HP.BP_Buff_HP_C" _returnvalue "Undefined" "OverrideRootScale" null null)
  ;[1 1 1] Генерация ловушек, которая зависит от количества пройденных комнат и от сложности предыдущей
  (bind _asbp_third_person_character (cast `/Game/ThirdPerson/Blueprints/BP_ThirdPersonCharacter` (`GameplayStatics.GetPlayerCharacter` 0)))
  (bind _counterofrooms (`/Game/ThirdPerson/Blueprints/BP_ThirdPersonCharacter.CounterOfRooms` _asbp_third_person_character))
  (bind _returnvalue_2 (+ _counterofrooms 2))
  (for _ (range (`KismetMathLibrary.RandomIntegerInRange` _returnvalue_2 _returnvalue_2) (+ (`KismetMathLibrary.RandomIntegerInRange` (+ _counterofrooms 7) (+ _counterofrooms 15)) 1))
    (`|SpawnActorFromClass` (`|GetArrayItem` (`self.Class_0`) (`KismetMathLibrary.RandomIntegerInRange` _counterofrooms (+ _counterofrooms 2))) _returnvalue "Undefined" "SelectDefaultAtRuntime" null null)))

(fn `UserConstructionScript`)