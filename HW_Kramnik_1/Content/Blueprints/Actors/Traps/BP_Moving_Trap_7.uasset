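; BP_Moving_Trap_7 is a rotating trap actor that subtracts damage from the third-person character's HP when overlapped.
; Damage and rotation speeds come from the Trap_7 row of DT_MovingTrap.
; Each tick it checks the player's IsAllSlower bonus flag and sets RotatingMovement to the table's minimum or maximum rate.
; The construction script sets the initial rotation rate from its Speed variable.
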(event `self.ReceiveActorBeginOverlap`
  (params (OtherActor :type "Actor Object Reference"))
  (bind _asbp_third_person_character (cast `/Game/ThirdPerson/Blueprints/BP_ThirdPersonCharacter` OtherActor))
  (bind _returnvalue (`|GetDataTableRow` "/Game/Blueprints/Actors/Traps/DataTable_MovingTrap/DT_MovingTrap.DT_MovingTrap" "Trap_7")
    (:`then`
      (set `/Game/ThirdPerson/Blueprints/BP_ThirdPersonCharacter.HP` (- (`/Game/ThirdPerson/Blueprints/BP_ThirdPersonCharacter.HP` _asbp_third_person_character) (`.Damage_6_654989FE4E63F363A3E9CA8EA5583D27` (break `/Game/Blueprints/Actors/Traps/DataTable_MovingTrap/BP_Structure` _returnvalue))) _asbp_third_person_character))))

(event `self.ReceiveTick`
  (params (DeltaSeconds :type "Float (single-precision)"))
  (bind _rotatingmovement (`self.RotatingMovement`))
  ;[1 1 1] Скорость движения, которая зависит от наличия бонуса.
  (bind _asbp_third_person_character (cast `/Game/ThirdPerson/Blueprints/BP_ThirdPersonCharacter` (`GameplayStatics.GetPlayerCharacter` 0)))
  (if (`/Game/ThirdPerson/Blueprints/BP_ThirdPersonCharacter.IsAllSlower?` _asbp_third_person_character)
    (bind _returnvalue (`|GetDataTableRow` "/Game/Blueprints/Actors/Traps/DataTable_MovingTrap/DT_MovingTrap.DT_MovingTrap" "Trap_7")
      (:`then`
        (set `RotatingMovementComponent.RotationRate` (`.Speed_of_rotation_Min_12_661941964A928688EC097A8E0B7D481B` (break `/Game/Blueprints/Actors/Traps/DataTable_MovingTrap/BP_Structure` _returnvalue)) _rotatingmovement)))
    (else
      (bind _returnvalue_2 (`|GetDataTableRow` "/Game/Blueprints/Actors/Traps/DataTable_MovingTrap/DT_MovingTrap.DT_MovingTrap" "Trap_7")
        (:`then`
          (set `RotatingMovementComponent.RotationRate` (`.Speed_of_rotation_Max_10_E9B7C66B406356E74664F28EC53BD716` (break `/Game/Blueprints/Actors/Traps/DataTable_MovingTrap/BP_Structure` _returnvalue_2)) _rotatingmovement))))))

(fn `UserConstructionScript`
  (set `RotatingMovementComponent.RotationRate` (`KismetMathLibrary.MakeRotator` 0.0 0.0 (`self.Speed`)) (`self.RotatingMovement`)))