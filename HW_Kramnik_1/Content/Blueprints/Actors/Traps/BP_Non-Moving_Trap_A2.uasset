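; BP_Non-Moving_Trap_A2 is a trap actor that damages the player character when an actor overlaps it.
; On overlap it casts player character 0 to BP_ThirdPersonCharacter, without checking which actor entered, and skips damage while that character is attacking or invulnerable.
; Otherwise it reads Damage from the Trap_2 row of DT_NonATrap, subtracts it directly from the character's HP and prints a debug string.
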(event `self.ReceiveActorBeginOverlap`
  (params (OtherActor :type "Actor Object Reference"))
  (bind _asbp_third_person_character (cast `/Game/ThirdPerson/Blueprints/BP_ThirdPersonCharacter` (`GameplayStatics.GetPlayerCharacter` 0)))
  (if (not (`/Game/ThirdPerson/Blueprints/BP_ThirdPersonCharacter.IsAttack?` _asbp_third_person_character))
    ;[1 1 1] Проверка на неуязвимость
    (if (not (`/Game/ThirdPerson/Blueprints/BP_ThirdPersonCharacter.IsInvulnerable?` _asbp_third_person_character))
      (bind _returnvalue (`|GetDataTableRow` "/Game/Blueprints/Actors/Traps/DataTable_Non-Moving_Trap_A/DT_NonATrap.DT_NonATrap" "Trap_2")
        (:`then`
          (set `/Game/ThirdPerson/Blueprints/BP_ThirdPersonCharacter.HP` (- (`/Game/ThirdPerson/Blueprints/BP_ThirdPersonCharacter.HP` _asbp_third_person_character) (`.Damage_2_067546534A5727F731C090BD3C4516FA` (break `/Game/Blueprints/Actors/Traps/DataTable_Non-Moving_Trap_A/BP_Structure_3` _returnvalue))) _asbp_third_person_character)
          (`KismetSystemLibrary.PrintString` "2"))))))

(fn `UserConstructionScript`)