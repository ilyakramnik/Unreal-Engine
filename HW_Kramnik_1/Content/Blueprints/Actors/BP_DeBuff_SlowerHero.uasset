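; BP_DeBuff_SlowerHero is a debuff pickup actor that damages and temporarily slows the player's BP_ThirdPersonCharacter when overlapped.
; On overlap it subtracts HP, destroys its Plane component and lowers the character's MaxWalkSpeed within a clamped range.
; After a short delay it adds the speed back under the same clamp, then destroys itself.
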(event `self.ReceiveActorBeginOverlap`
  (params (OtherActor :type "Actor Object Reference"))
  (bind _asbp_third_person_character (cast `/Game/ThirdPerson/Blueprints/BP_ThirdPersonCharacter` OtherActor))
  (set `/Game/ThirdPerson/Blueprints/BP_ThirdPersonCharacter.HP` (- (`/Game/ThirdPerson/Blueprints/BP_ThirdPersonCharacter.HP` _asbp_third_person_character) 100.0) _asbp_third_person_character)
  (`ActorComponent.K2_DestroyComponent` (`self.Plane`))
  (bind _charactermovement (`Character.CharacterMovement` _asbp_third_person_character))
  (set `CharacterMovementComponent.MaxWalkSpeed` (`KismetMathLibrary.FClamp` (- (`CharacterMovementComponent.MaxWalkSpeed` _charactermovement) 300.0) 300.0 600.0) _charactermovement)
  (`KismetSystemLibrary.Delay` 5.0)
  (bind _charactermovement_2 (`Character.CharacterMovement` _asbp_third_person_character))
  (set `CharacterMovementComponent.MaxWalkSpeed` (`KismetMathLibrary.FClamp` (+ (`CharacterMovementComponent.MaxWalkSpeed` _charactermovement_2) 300.0) 300.0 600.0) _charactermovement_2)
  (`self.K2_DestroyActor`))

(fn `UserConstructionScript`)