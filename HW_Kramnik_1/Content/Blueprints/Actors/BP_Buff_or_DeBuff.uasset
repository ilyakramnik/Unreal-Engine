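; A pickup actor that randomly gives the overlapping third-person character either a temporary buff or a debuff.
; On overlap it destroys its Cube component, then picks one of two outcomes with equal chance.
; The debuff lowers max walk speed for a fixed delay, while the shield buff sets IsInvulnerable for the Time variable's duration.
; After the delay it reverts the change and destroys itself.
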(event `self.ReceiveActorBeginOverlap`
  (params (OtherActor :type "Actor Object Reference"))
  (bind _asbp_third_person_character (cast `/Game/ThirdPerson/Blueprints/BP_ThirdPersonCharacter` OtherActor))
  (`ActorComponent.K2_DestroyComponent` (`self.Cube`))
  (if (== (`KismetMathLibrary.RandomIntegerInRange` 0 1) 0)
    (bind _charactermovement (`Character.CharacterMovement` _asbp_third_person_character))
    ;[1 1 1] Дебафф замедления
    (set `CharacterMovementComponent.MaxWalkSpeed` (- (`CharacterMovementComponent.MaxWalkSpeed` _charactermovement) 300.0) _charactermovement)
    (`KismetSystemLibrary.Delay` 5.0)
    (bind _charactermovement_2 (`Character.CharacterMovement` _asbp_third_person_character))
    (set `CharacterMovementComponent.MaxWalkSpeed` (+ (`CharacterMovementComponent.MaxWalkSpeed` _charactermovement_2) 300.0) _charactermovement_2)
    (`self.K2_DestroyActor`)
    (else
      ;[1 1 1] Бафф щита
      (set `/Game/ThirdPerson/Blueprints/BP_ThirdPersonCharacter.IsInvulnerable?` true _asbp_third_person_character)
      (`KismetSystemLibrary.Delay` (`self.time`))
      (set `/Game/ThirdPerson/Blueprints/BP_ThirdPersonCharacter.IsInvulnerable?` false _asbp_third_person_character)
      (`self.K2_DestroyActor`))))

(fn `UserConstructionScript`)