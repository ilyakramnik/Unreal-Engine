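; Pickup buff actor that switches on a temporary "all slower" state when a BP_ThirdPersonCharacter overlaps it.
; On overlap it destroys its three cube components and sets IsAllSlower on the character.
; The actor stays alive through a delay of Time, then clears the flag and destroys itself.
; The slowing effect itself is not implemented here, only the flag toggle.
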(event `self.ReceiveActorBeginOverlap`
  (params (OtherActor :type "Actor Object Reference"))
  (bind _asbp_third_person_character (cast `/Game/ThirdPerson/Blueprints/BP_ThirdPersonCharacter` OtherActor))
  (`ActorComponent.K2_DestroyComponent` (`self.Cube1`))
  (`ActorComponent.K2_DestroyComponent` (`self.Cube`))
  (`ActorComponent.K2_DestroyComponent` (`self.Cube2`))
  (set `/Game/ThirdPerson/Blueprints/BP_ThirdPersonCharacter.IsAllSlower?` true _asbp_third_person_character)
  (`KismetSystemLibrary.Delay` (`self.time`))
  (set `/Game/ThirdPerson/Blueprints/BP_ThirdPersonCharacter.IsAllSlower?` false _asbp_third_person_character)
  (`self.K2_DestroyActor`))

(fn `UserConstructionScript`)